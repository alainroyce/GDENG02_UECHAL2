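; Breakable cylinder actor, apparently a fracture prop, that drops a random upgrade when hit.
; The first Hit event passes a DoOnce, plays a collapse sound at the world origin and waits briefly.
; It then spawns a cube, cone, cylinder or capsule upgrade Blueprint at its own location, chosen by a random integer switch.
; The actor is not destroyed in this graph.
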(event EventBeginPlay)

(event Collision|EventActorBeginOverlap
  (params (OtherActor :type Actor%20Object%20Reference)))

(event EventTick
  (params (DeltaSeconds :type Float%20%28single-precision%29)))

(event Collision|EventHit
  (params (MyComp :type Primitive%20Component%20Object%20Reference) (Other :type Actor%20Object%20Reference) (OtherComp :type Primitive%20Component%20Object%20Reference) (bSelfMoved :type Boolean) (HitLocation :type Vector :default "0, 0, 0") (HitNormal :type Vector :default "0, 0, 0") (NormalImpulse :type Vector :default "0, 0, 0") (Hit :type Hit%20Result%20Structure%20%28by%20ref%29))
  (bind _self self)
  (bind _returnvalue (Transformation|GetActorLocation _self))
  (bind _returnvalue_2 (Math|Conversions|ToTransform(Vector) _returnvalue))
  (Utilities|FlowControl|DoOnce false
    (:Completed
      (Audio|PlaySoundatLocation "/Game/StarterContent/Audio/Collapse01.Collapse01" "0, 0, 0" "0, 0, 0" 1.0 1.0 0.0 0 0 0 0)
      (Utilities|FlowControl|Delay 0.2)
      (switch int (Math|Random|RandomIntegerinRange 0 3)
        (:Default
          (Game|SpawnActorfromClass "/Game/Upgrades/CubeUpgrade_Blueprint.CubeUpgrade_Blueprint_C" _returnvalue_2 "Undefined" 0 0 :!label _label))
        (:0
          (goto _label))
        (:1
          (Game|SpawnActorfromClass "/Game/Upgrades/ConeUpgrade_Blueprint.ConeUpgrade_Blueprint_C" _returnvalue_2 "Undefined" 0 0))
        (:2
          (Game|SpawnActorfromClass "/Game/Upgrades/CylinderUpgrade_Blueprint.CylinderUpgrade_Blueprint_C" _returnvalue_2 "Undefined" 0 0))
        (:3
          (Game|SpawnActorfromClass "/Game/Upgrades/CapsuleUpgrade_Blueprint.CapsuleUpgrade_Blueprint_C" _returnvalue_2 "Undefined" 0 0))))))

(fn ConstructionScript)